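; BP_WaveSpawner runs enemy waves, starting the first on BeginPlay and showing a success screen when none remain.
; SpawnWave plays a sound, reads the current wave's enemy count from the Waves map values, and spawns that many BP_Enemy actors at random SpawnPositions.
; CheckForEnemies waits briefly, then starts the next wave if no enemies are left.
; After the last wave, it clears all widgets, shows the Success widget and enables the mouse cursor.
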(event Custom|Spawn%20Wave
  (bind _returnvalue (Game|GetPlayerController 0))
  (bind _current_wave (Variables|Default|GetCurrent%20Wave))
  (Audio|PlaySound2D "/Game/Audio/Wave.Wave" 1.0 1.0 0.0 0 0)
  (if (<= (+ _current_wave 1) (Utilities|Map|Length (Variables|Default|GetWaves)))
    (Math|Integer|IncrementInt _current_wave
      (:%20%20
        (bind _values (Utilities|Map|Values (Variables|Default|GetWaves)))
        (for _index (range 1 (Utilities|Array|Get(acopy) _values (- (Variables|Default|GetCurrent%20Wave) 1)))
          (Game|SpawnActorfromClass "/Game/Blueprint/BP_Enemy.BP_Enemy_C" (.OutItem (Utilities|Array|Random (Variables|Default|GetSpawn%20Positions))) "AlwaysSpawn" "MultiplyWithRoot" 0 0))))
    (else
      (Viewport|RemoveAllWidgets)
      (bind _returnvalue_2 (UserInterface|CreateWidget "/Game/UI/success.success_C" _returnvalue))
      (UserInterface|Viewport|AddtoViewport _returnvalue_2 0)
      (Variables|/Script/Engine.PlayerController|SetbShowMouseCursor _returnvalue true))))

(event Custom|Check%20For%20Enemies
  (Utilities|FlowControl|Delay 0.2)
  (bind _outactors (Actor|GetAllActorsOfClass "/Game/Blueprint/BP_Enemy.BP_Enemy_C"))
  (if (<= (Utilities|Array|Length _outactors) 0)
    (CallFunction|SpawnWave)))

(event EventBeginPlay
  (CallFunction|SpawnWave))

(fn ConstructionScript)